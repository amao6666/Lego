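; Enemy AI controller that turns perception events into blackboard data.
; Successfully sensed stimuli tagged "Noise" write their location to the NoisePos key.
; Any other sensed stimulus, treated as sight, stores the actor as Target only while no valid target is set.
; Lost stimuli are ignored, so this graph never clears either key, and both branches print debug strings.
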(event `self.PerceptionComponent.OnTargetPerceptionUpdated`
  (params (Actor :type "Actor Object Reference") (Stimulus :type "AIStimulus Structure"))
  (bind (_age _expirationage _strength _stimuluslocation _receiverlocation _tag _bsuccessfullysensed) (break `AIStimulus` Stimulus))
  (bind _returnvalue (`AIBlueprintHelperLibrary.GetBlackboard` null))
  (if _bsuccessfullysensed
    (if (== _tag "Noise")
      (`BlackboardComponent.SetValueAsVector` _returnvalue (`self.NoisePos`) _stimuluslocation)
      (`KismetSystemLibrary.PrintString` "Noise")
      (else
        (`/Engine/EditorBlueprintResources/StandardMacros.IsValid` (`BlackboardComponent.GetValueAsObject` _returnvalue (`self.Target`))
          (:`Is Not Valid`
            (`BlackboardComponent.SetValueAsObject` _returnvalue (`self.Target`) Actor)
            (`KismetSystemLibrary.PrintString` "Sight")))))))

(fn `UserConstructionScript`)